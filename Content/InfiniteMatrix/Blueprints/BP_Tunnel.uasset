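; Tunnel segment for an endless flying shooter, with a rotating holed wall and optional medkit and enemy.
; Crossing the trigger zone adds score and speed, has TunnelSpawner spawn another tunnel, then destroys this one.
; Overlaps apply damage with camera shake or restart at zero health, heal via medkit, or let projectiles kill enemies for score.
; Randomize functions pick wall mesh and roll, and randomly remove or offset the medkit and enemy.
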(event `self.ReceiveTick`
  (params (DeltaSeconds :type "Float (single-precision)"))
  (if (not (`self.WallmeshDestroyed`))
    (`SceneComponent.K2_AddLocalRotation` (`self.WallMesh`) (`KismetMathLibrary.MakeRotator` (* DeltaSeconds (`self.RotateSpeed`))) false false)))

(event `self.TriggerZone.OnComponentBeginOverlap`
  (params (OverlappedComponent :type "PrimitiveComponent Object Reference") (OtherActor :type "Actor Object Reference") (OtherComp :type "PrimitiveComponent Object Reference") (OtherBodyIndex :type Integer) (bFromSweep :type Boolean) (SweepResult :type "HitResult Structure (by ref)"))
  (bind _asbp_player (cast `/Game/InfiniteMatrix/Blueprints/BP_Player` OtherActor))
  (set `/Game/InfiniteMatrix/Blueprints/BP_Player.Score` (+ (`/Game/InfiniteMatrix/Blueprints/BP_Player.Score` _asbp_player) 1) _asbp_player)
  (set `/Game/InfiniteMatrix/Blueprints/BP_Player.ForwardSpeed` (`KismetMathLibrary.FClamp` (+ (`/Game/InfiniteMatrix/Blueprints/BP_Player.ForwardSpeed` _asbp_player) 20.0) 1000.0 3000.0) _asbp_player)
  (`/Game/InfiniteMatrix/Blueprints/BP_TunnelSpawner.SpawnTunnelAtSpawnPoint` (`self.TunnelSpawner`))
  (`self.K2_DestroyActor`))

(event `self.WallMesh.OnComponentBeginOverlap`
  (params (OverlappedComponent :type "PrimitiveComponent Object Reference") (OtherActor :type "Actor Object Reference") (OtherComp :type "PrimitiveComponent Object Reference") (OtherBodyIndex :type Integer) (bFromSweep :type Boolean) (SweepResult :type "HitResult Structure (by ref)"))
  (bind _asbp_player (cast `/Game/InfiniteMatrix/Blueprints/BP_Player` OtherActor)
    (:`then`
      (set `/Game/InfiniteMatrix/Blueprints/BP_Player.Health` (`KismetMathLibrary.FClamp` (- (`/Game/InfiniteMatrix/Blueprints/BP_Player.Health` _asbp_player) 20.0) 0.0 100.0) _asbp_player)
      (`ActorComponent.K2_DestroyComponent` OverlappedComponent)
      (set `self.WallmeshDestroyed` true)
      (if (== (`/Game/InfiniteMatrix/Blueprints/BP_Player.Health` _asbp_player) 0.0)
        (`/Game/InfiniteMatrix/Blueprints/BP_Player.DisplayRestart` _asbp_player)
        (else
          (`GameplayStatics.PlayWorldCameraShake` "/Game/InfiniteMatrix/Blueprints/BP_CameraShake.BP_CameraShake_C" (`self.K2_GetActorLocation` (`GameplayStatics.GetPlayerPawn` 0)) 0.0 500.0))))
    (:`CastFailed`
      (bind _asbp_projectile (cast `/Game/InfiniteMatrix/Blueprints/BP_Projectile` OtherActor))
      (if (not (`/Game/InfiniteMatrix/Blueprints/BP_Projectile.ProjectileDestroyed` _asbp_projectile))
        (set `/Game/InfiniteMatrix/Blueprints/BP_Projectile.ProjectileDestroyed` true _asbp_projectile)
        (`self.K2_DestroyActor` _asbp_projectile)))))

(event `self.MedkitMesh.OnComponentBeginOverlap`
  (params (OverlappedComponent :type "PrimitiveComponent Object Reference") (OtherActor :type "Actor Object Reference") (OtherComp :type "PrimitiveComponent Object Reference") (OtherBodyIndex :type Integer) (bFromSweep :type Boolean) (SweepResult :type "HitResult Structure (by ref)"))
  (bind _asbp_player (cast `/Game/InfiniteMatrix/Blueprints/BP_Player` OtherActor))
  (if (not (`self.MedkitDestroyed`))
    (`ActorComponent.K2_DestroyComponent` OverlappedComponent)
    (set `/Game/InfiniteMatrix/Blueprints/BP_Player.Health` (`KismetMathLibrary.FClamp` (+ (`/Game/InfiniteMatrix/Blueprints/BP_Player.Health` _asbp_player) 15.0) 0.0 100.0) _asbp_player)))

(event `self.EnemyMesh.OnComponentBeginOverlap`
  (params (OverlappedComponent :type "PrimitiveComponent Object Reference") (OtherActor :type "Actor Object Reference") (OtherComp :type "PrimitiveComponent Object Reference") (OtherBodyIndex :type Integer) (bFromSweep :type Boolean) (SweepResult :type "HitResult Structure (by ref)"))
  (bind _asbp_player (cast `/Game/InfiniteMatrix/Blueprints/BP_Player` OtherActor)
    (:`then`
      (`ActorComponent.K2_DestroyComponent` OverlappedComponent)
      (set `/Game/InfiniteMatrix/Blueprints/BP_Player.Health` (`KismetMathLibrary.FClamp` (- (`/Game/InfiniteMatrix/Blueprints/BP_Player.Health` _asbp_player) 20.0) 0.0 100.0) _asbp_player)
      (if (== (`/Game/InfiniteMatrix/Blueprints/BP_Player.Health` _asbp_player) 0.0)
        (`/Game/InfiniteMatrix/Blueprints/BP_Player.DisplayRestart` _asbp_player)
        (else
          (`GameplayStatics.PlayWorldCameraShake` "/Game/InfiniteMatrix/Blueprints/BP_CameraShake.BP_CameraShake_C" (`self.K2_GetActorLocation` (`GameplayStatics.GetPlayerPawn` 0)) 0.0 500.0))))
    (:`CastFailed`
      (bind _asbp_projectile (cast `/Game/InfiniteMatrix/Blueprints/BP_Projectile` OtherActor))
      (if (not (`/Game/InfiniteMatrix/Blueprints/BP_Projectile.ProjectileDestroyed` _asbp_projectile))
        (set `/Game/InfiniteMatrix/Blueprints/BP_Projectile.ProjectileDestroyed` true _asbp_projectile)
        (if (not (`self.EnemyDestroyed`))
          (set `self.EnemyDestroyed` true)
          (`ActorComponent.K2_DestroyComponent` OverlappedComponent)
          (`self.K2_DestroyActor` _asbp_projectile)
          (bind _returnvalue (`GameplayStatics.GetActorOfClass` "/Game/InfiniteMatrix/Blueprints/BP_Player.BP_Player_C"))
          (set `/Game/InfiniteMatrix/Blueprints/BP_Player.Score` (+ (`/Game/InfiniteMatrix/Blueprints/BP_Player.Score` _returnvalue) 1) _returnvalue))))))

(fn `RandomizeEnemy`
  (bind _enemymesh (`self.EnemyMesh`))
  (if (`self.EnemyDestroyed`)
    _
    (elif (> (`KismetMathLibrary.RandomIntegerInRange` 1 10) 5)
      (`ActorComponent.K2_DestroyComponent` _enemymesh)
      (else
        (`SceneComponent.K2_AddLocalOffset` _enemymesh (`KismetMathLibrary.MakeVector` (`KismetMathLibrary.RandomFloatInRange` -300.0 300.0) (`KismetMathLibrary.RandomFloatInRange` -2000.0 -1500.0) (`KismetMathLibrary.RandomFloatInRange` -300.0 300.0)) false false)))))

(fn `RandomizeMedkit`
  (bind _medkitmesh (`self.MedkitMesh`))
  (if (`self.MedkitDestroyed`)
    _
    (elif (!= (`KismetMathLibrary.RandomIntegerInRange` 1 10) 1)
      (`ActorComponent.K2_DestroyComponent` _medkitmesh)
      (else
        (`SceneComponent.K2_AddLocalOffset` _medkitmesh (`KismetMathLibrary.MakeVector` (`KismetMathLibrary.RandomFloatInRange` -300.0 300.0) (`KismetMathLibrary.RandomFloatInRange` -2000.0 -1500.0) (`KismetMathLibrary.RandomFloatInRange` -300.0 300.0)) false false)))))

(fn `RandomizeWall`
  (`StaticMeshComponent.SetStaticMesh` (`self.WallMesh`) (select `int` (`KismetMathLibrary.RandomIntegerInRange` 0 3) :`0` "/Game/InfiniteMatrix/Meshes/SM_Hole_01.SM_Hole_01" :`1` "/Game/InfiniteMatrix/Meshes/SM_Hole_02.SM_Hole_02" :`2` "/Game/InfiniteMatrix/Meshes/SM_Hole_03.SM_Hole_03" :`3` "/Game/InfiniteMatrix/Meshes/SM_Hole_04.SM_Hole_04" :!type "StaticMesh Object Reference"))
  (`SceneComponent.K2_AddLocalRotation` (`self.WallMesh`) (`KismetMathLibrary.MakeRotator` (`KismetMathLibrary.RandomFloatInRange` 0.0 360.0)) false false))

(fn `UserConstructionScript`)